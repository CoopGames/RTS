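; CameraPawn is an RTS camera pawn Blueprint that currently only probes for surfaces along its scene component's up axis.
; Each Tick it line-traces 500 units along Scene1's up vector on the Visibility channel, with debug drawing, and prints the hit's Z.
; Unconnected logic would cap the camera's height at 100 or snap the actor to the hit location, but neither runs.
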(event EventBeginPlay
  (Variables|Default|SetWorldScene (Variables|Default|GetScene1)))

(event Collision|EventActorBeginOverlap
  (params (OtherActor :type Actor%20Object%20Reference)))

(event EventTick
  (params (DeltaSeconds :type Float%20%28single-precision%29))
  (bind _scene1 (Variables|Default|GetScene1))
  (bind _returnvalue (Transformation|GetWorldLocation _scene1))
  (bind (_outhit _returnvalue_2) (Collision|LineTraceByChannel _returnvalue (+ _returnvalue (* (Math|Vector|GetUpVector _scene1) 5e+02)) "TraceTypeQuery1" false 0 "ForDuration"))
  (if _returnvalue_2
    (Development|PrintString (Utilities|String|ToString(Float) (.Z (Math|Vector|BreakVector (.Location (Collision|BreakHitResult _outhit))))))))

(fn ConstructionScript)