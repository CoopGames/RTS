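; Selection-rectangle actor ("AuswahlQuadrat") for the RTS, pairing a Box component with a visual area.
; ReDrawArea converts a world position into the Scene component's local space and divides it by a fixed factor.
; The result serves as both offset and half-size, so the box grows from the origin toward that point.
; The visual follows with signed, flattened scale, while the box extent uses absolute values.
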(event EventBeginPlay)

(event Collision|EventActorBeginOverlap
  (params (OtherActor :type Actor%20Object%20Reference)))

(event EventTick
  (params (DeltaSeconds :type Float%20%28single-precision%29)))

(fn ConstructionScript)

(fn ReDrawArea
  (params (AreaPosition :type Vector))
  (bind _visualareaparent (Variables|Default|GetVisualAreaParent))
  (Variables|Default|SetPosition (Math|Transform|InverseTransformLocation (Transformation|GetWorldTransform (Variables|Default|GetScene)) AreaPosition))
  (Variables|Default|SetPosition (/ (Variables|Default|GetPosition) 3.5))
  (Components|Box|SetBoxExtent (Variables|Default|GetBox) (Math|Vector|MakeVector (Math|Float|Absolute(Float) (.X (Math|Vector|BreakVector (Variables|Default|GetPosition)))) (Math|Float|Absolute(Float) (.Y (Math|Vector|BreakVector (Variables|Default|GetPosition)))) 1.0) true)
  (Transformation|SetRelativeLocation (Variables|Default|GetBox) (Variables|Default|GetPosition) false false)
  (Transformation|SetRelativeLocation _visualareaparent (Variables|Default|GetPosition) false false)
  (Transformation|SetRelativeScale3D _visualareaparent (Math|Vector|MakeVector (/ (.X (Math|Vector|BreakVector (Variables|Default|GetPosition))) 32.0) (/ (.Y (Math|Vector|BreakVector (Variables|Default|GetPosition))) 32.0) 0.0)))