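; Base building actor for the RTS that applies its configured mesh and registers with the player's RTS camera controller on begin play.
; Residential buildings (Wohnhaus) report their housing space and money cost to the controller when placed.
; It binds to the controller's HUD request and, when requested for itself, replaces the HUD's info window with a GebäudeInfo widget.
; Utility-building placement and resource-cost checks are present but unconnected.
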(event Custom|ErstelleInfofenster
  (params (Actor :type Actor%20Object%20Reference))
  (bind _commander (Variables|Default|GetCommander))
  (bind _mainhudref (Variables|/Game/RTS/Blueprints/RTSCameraController.RTSCameraController_C|GetMainHUDRef _commander))
  (if (== Actor self)
    (bind _returnvalue (UserInterface|CreateWidget "/Game/RTS/UIS/GebäudeInfo.GebäudeInfo_C" (Game|GetPlayerController 0) (Variables|Default|GetGebäudeType) self))
    (Default|LöscheInfoFenster _mainhudref)
    (Widget|Panel|AddChild (Variables|/Game/RTS/UIS/MainUI_HUD.MainUI_HUD_C|GetInformationen _mainhudref) _returnvalue)))

(event EventBeginPlay
  (Components|StaticMesh|SetStaticMesh (Variables|Debug|GetStaticMeshComponent) (Variables|Default|GetActualActor))
  (bind _asrtscamera_controller (Utilities|Casting|CastToRTSCameraController (Game|GetPlayerController 0)))
  (Variables|Default|SetCommander _asrtscamera_controller)
  (EventDispatchers|BindEventtoHUDRequest (Variables|Default|GetCommander) (EventDispatchers|CreateEvent :!event Custom|ErstelleInfofenster))
  (switch Utilities|FlowControl|Switch|SwitchonGebäudeTypes (Variables|Default|GetGebäudeType)
    (:NewEnumerator0
      (Default|PlatziereWohngebäude (Variables|Default|GetCommander) (Variables|Default|GetWohnraum) (Variables|Default|GetGeldKosten)))))

(event Collision|EventActorBeginOverlap
  (params (OtherActor :type Actor%20Object%20Reference)))

(event EventTick
  (params (DeltaSeconds :type Float%20%28single-precision%29)))

(fn ConstructionScript)