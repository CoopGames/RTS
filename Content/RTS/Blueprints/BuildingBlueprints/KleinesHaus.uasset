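; KleinesHaus is the Blueprint for a small residential building in the RTS game.
; On BeginPlay it casts player controller 0 to RTSCameraController, stores it as Commander, and calls PlatziereWohngebäude with its Wohnraum (housing space) and Kosten (cost) values.
; Any effect on housing or resources is left to the controller.
; SetCalendar and SetClock are stubs returning false, and the construction script is empty.
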(event EventBeginPlay
  (bind _asrtscamera_controller (Utilities|Casting|CastToRTSCameraController (Game|GetPlayerController 0)))
  (Variables|Default|SetCommander _asrtscamera_controller)
  (Default|PlatziereWohngebäude (Variables|Default|GetCommander) (Variables|Default|GetWohnraum) (Variables|Default|GetKosten)))

(event Collision|EventActorBeginOverlap
  (params (OtherActor :type Actor%20Object%20Reference)))

(event EventTick
  (params (DeltaSeconds :type Float%20%28single-precision%29)))

(fn ConstructionScript)

(fn SetCalendar
  (params (Date :type Array%20of%20Integers))
  (return false))

(fn SetClock
  (params (Time :type Array%20of%20Integers))
  (return false))