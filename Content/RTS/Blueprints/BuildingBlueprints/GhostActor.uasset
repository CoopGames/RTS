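; GhostActor is the placement preview for a building in the RTS, showing the ghost mesh from its GebäudeStruct.
; On BeginPlay it caches the RTSCameraController as Commander, then each Tick asks it whether the building's money cost is affordable and sets PlatzierenNichtMöglich (placement not possible) accordingly.
; Overlapping a GebäudeActor swaps to the red mesh and sets the Commander's BadTerrain flag; any end overlap restores both.
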(event EventBeginPlay
  (Components|StaticMesh|SetStaticMesh (Variables|Debug|GetStaticMeshComponent) (.GhostActor (Utilities|Struct|BreakGebäudeDatenBankStruktur (Variables|Default|GetGebäudeStruct))))
  (bind _asrtscamera_controller (Utilities|Casting|CastToRTSCameraController (Game|GetPlayerController 0)))
  (Variables|Default|SetCommander _asrtscamera_controller))

(event EventTick
  (params (DeltaSeconds :type Float%20%28single-precision%29))
  (bind _commander (Variables|Default|GetCommander))
  (bind _genug_ (Default|ÜberprüfeGeld (Variables|Default|GetCommander) (.GeldKosten (Utilities|Struct|BreakGebäudeDatenBankStruktur (Variables|Default|GetGebäudeStruct)))))
  (if _genug_
    (Default|PlatzierenNichtMöglich? _commander false)
    (else
      (Default|PlatzierenNichtMöglich? _commander true))))

(event Collision|EventActorBeginOverlap
  (params (OtherActor :type Actor%20Object%20Reference))
  (if (== (Utilities|GetClass OtherActor) "/Game/RTS/Blueprints/BuildingBlueprints/GebäudeActor.GebäudeActor_C")
    (Components|StaticMesh|SetStaticMesh (Variables|Debug|GetStaticMeshComponent) (.OverlappingRed (Utilities|Struct|BreakGebäudeDatenBankStruktur (Variables|Default|GetGebäudeStruct))))
    (Variables|/Game/RTS/Blueprints/RTSCameraController.RTSCameraController_C|SetBadTerrain (Variables|Default|GetCommander) true)))

(event Collision|EventActorEndOverlap
  (params (OtherActor :type Actor%20Object%20Reference))
  (Components|StaticMesh|SetStaticMesh (Variables|Debug|GetStaticMeshComponent) (.GhostActor (Utilities|Struct|BreakGebäudeDatenBankStruktur (Variables|Default|GetGebäudeStruct))))
  (Variables|/Game/RTS/Blueprints/RTSCameraController.RTSCameraController_C|SetBadTerrain (Variables|Default|GetCommander) false))

(fn ConstructionScript)