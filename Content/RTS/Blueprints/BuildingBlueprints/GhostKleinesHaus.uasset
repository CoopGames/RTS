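; Placement ghost for a small house (Kleines Haus) in the RTS, showing whether the current spot is blocked.
; Beginning an overlap switches the mesh to copper and sets BadTerrain on the commander's RTSCameraController; ending one restores glass and clears the flag.
; Overlaps are not counted, so leaving any one actor clears the blocked state.
; IAmYourCommander has no logic of its own, and SetCalendar and SetClock are stubs returning false.
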(event EventBeginPlay)

(event EventIAmYourCommander
  (params (Commander :type Actor%20Object%20Reference)))

(event EventTick
  (params (DeltaSeconds :type Float%20%28single-precision%29)))

(event Collision|EventActorBeginOverlap
  (params (OtherActor :type Actor%20Object%20Reference))
  (Rendering|Material|SetMaterial (Variables|Debug|GetStaticMeshComponent) 0 "/Game/StarterContent/Materials/M_Metal_Copper.M_Metal_Copper")
  (bind _asrtscamera_controller (Utilities|Casting|CastToRTSCameraController (stale EventIAmYourCommander Commander)))
  (Variables|/Game/RTS/Blueprints/RTSCameraController.RTSCameraController_C|SetBadTerrain _asrtscamera_controller true))

(event Collision|EventActorEndOverlap
  (params (OtherActor :type Actor%20Object%20Reference))
  (Rendering|Material|SetMaterial (Variables|Debug|GetStaticMeshComponent) 0 "/Game/StarterContent/Materials/M_Glass.M_Glass")
  (bind _asrtscamera_controller (Utilities|Casting|CastToRTSCameraController (stale EventIAmYourCommander Commander)))
  (Variables|/Game/RTS/Blueprints/RTSCameraController.RTSCameraController_C|SetBadTerrain _asrtscamera_controller false))

(fn ConstructionScript)

(fn SetCalendar
  (params (Date :type Array%20of%20Integers))
  (return false))

(fn SetClock
  (params (Time :type Array%20of%20Integers))
  (return false))