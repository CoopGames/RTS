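; Placement ghost for the medium house in the RTS, previewing the building and telling the RTSCameraController whether it can be placed.
; Every tick it checks affordability of Kosten and sets the controller's placement-blocked flag.
; Overlaps swap the mesh from glass to copper and block placement, but Tick rewrites the same flag, so affordability overrides the overlap block.
; SetCalendar and SetClock are stubs returning false.
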(event EventBeginPlay
  (bind _asrtscamera_controller (Utilities|Casting|CastToRTSCameraController (Game|GetPlayerController 0)))
  (Variables|Default|SetCommander _asrtscamera_controller))

(event EventTick
  (params (DeltaSeconds :type Float%20%28single-precision%29))
  (bind _genug_ (Default|ÜberprüfeGeld (Variables|Default|GetCommander) (Variables|Default|GetKosten)))
  (if _genug_
    (Default|PlatzierenNichtMöglich? (Variables|Default|GetCommander) false)
    (else
      (Default|PlatzierenNichtMöglich? (Variables|Default|GetCommander) true))))

(event Collision|EventActorBeginOverlap
  (params (OtherActor :type Actor%20Object%20Reference))
  (Rendering|Material|SetMaterial (Variables|Debug|GetStaticMeshComponent) 0 "/Game/StarterContent/Materials/M_Metal_Copper.M_Metal_Copper")
  (Default|PlatzierenNichtMöglich? (Variables|Default|GetCommander) true))

(event Collision|EventActorEndOverlap
  (params (OtherActor :type Actor%20Object%20Reference))
  (Rendering|Material|SetMaterial (Variables|Debug|GetStaticMeshComponent) 0 "/Game/StarterContent/Materials/M_Glass.M_Glass")
  (Default|PlatzierenNichtMöglich? (Variables|Default|GetCommander) false))

(fn ConstructionScript)

(fn SetCalendar
  (params (Date :type Array%20of%20Integers))
  (return false))

(fn SetClock
  (params (Time :type Array%20of%20Integers))
  (return false))