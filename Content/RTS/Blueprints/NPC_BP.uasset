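; NPC Blueprint for an RTS that sets up a villager's profession look and profile when play begins.
; RandomNPCFeatures creates a dynamic material on the mesh and tints BodyColor by profession, such as farmer, fisher, miner or smith.
; It then stores a profile struct holding a random name and the profession, which fills the Gender field.
; GetRandomName always draws from the male name enum; the female branch is never reached.
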(event EventBeginPlay
  (CallFunction|RandomNPCFeatures (Variables|Default|GetType)))

(event Collision|EventActorBeginOverlap
  (params (OtherActor :type Actor%20Object%20Reference)))

(event EventTick
  (params (DeltaSeconds :type Float%20%28single-precision%29)))

(fn ConstructionScript)

(fn RandomNPCFeatures
  (params (Type :type NPCType%20Enum :default "NewEnumerator0"))
  (Variables|Default|SetNPCType Type)
  (bind _returnvalue (Rendering|Material|CreateDynamicMaterialInstance (Variables|Character|GetMesh) 0 "/Game/RTS/Character/Materials/M_UE4Man_Body_Inst.M_UE4Man_Body_Inst" :!class /Script/Engine.PrimitiveComponent))
  (LocalVariables|SetMaterialInstance _returnvalue)
  (switch Utilities|FlowControl|Switch|SwitchonNPCType (Variables|Default|GetNPCType)
    (:NewEnumerator0
      (Rendering|Material|SetVectorParameterValue (LocalVariables|GetMaterialInstance) "BodyColor" "(R=1.000000,G=0.902706,B=0.000000,A=1.000000)" :!class /Script/Engine.MaterialInstanceDynamic))
    (:NewEnumerator2
      (Rendering|Material|SetVectorParameterValue (LocalVariables|GetMaterialInstance) "BodyColor" "(R=1.000000,G=0.142180,B=0.000000,A=1.000000)" :!class /Script/Engine.MaterialInstanceDynamic))
    (:NewEnumerator9
      (Rendering|Material|SetVectorParameterValue (LocalVariables|GetMaterialInstance) "BodyColor" "(R=0.006859,G=0.600335,B=1.000000,A=1.000000)" :!class /Script/Engine.MaterialInstanceDynamic))
    (:NewEnumerator3
      (Rendering|Material|SetVectorParameterValue (LocalVariables|GetMaterialInstance) "BodyColor" "(R=0.166667,G=0.166667,B=0.166667,A=1.000000)" :!class /Script/Engine.MaterialInstanceDynamic))
    (:NewEnumerator10
      (Rendering|Material|SetVectorParameterValue (LocalVariables|GetMaterialInstance) "BodyColor" "(R=0.879066,G=1.000000,B=0.354167,A=1.000000)" :!class /Script/Engine.MaterialInstanceDynamic))
    (:NewEnumerator11
      (Rendering|Material|SetVectorParameterValue (LocalVariables|GetMaterialInstance) "BodyColor" "(R=1.000000,G=0.016950,B=0.000000,A=1.000000)" :!class /Script/Engine.MaterialInstanceDynamic))
    (:NewEnumerator12
      (Rendering|Material|SetVectorParameterValue (LocalVariables|GetMaterialInstance) "BodyColor" "(R=0.000000,G=1.000000,B=0.056642,A=1.000000)" :!class /Script/Engine.MaterialInstanceDynamic))
    (:NewEnumerator13
      (Rendering|Material|SetVectorParameterValue (LocalVariables|GetMaterialInstance) "BodyColor" "(R=0.005208,G=0.005208,B=0.005208,A=1.000000)" :!class /Script/Engine.MaterialInstanceDynamic)))
  (bind _name (CallFunction|GetRandomName "NewEnumerator0"))
  (Variables|Default|SetMyProfile (Utilities|Struct|MakeNPCProfile_struct _name (Variables|Default|GetNPCType))))

(fn GetRandomName
  (params (Gender :type NPCType%20Enum :default "NewEnumerator0"))
  (return (Utilities|String|EnumtoString (Utilities|Enum|LiteralenumNPCNameMale (Utilities|Enum|ByteToEnumNPCNameMale (Math|Conversions|ToByte(Integer) (Math|Random|RandomIntegerinRange 0 (- (|GetNumEnumEntries) 1))))))))