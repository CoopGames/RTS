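; RTS player controller that drives the camera pawn and handles building placement, selection and time controls for a city-builder style game.
; Camera input covers zoom-scaled axis movement, screen-edge scrolling, gated pan rotation and spring-arm zoom.
; Buildings come from a data table as a cursor-following ghost, rotated by wheel and spawned on click unless terrain is bad.
; It also creates the main HUD, updates resources, spawns NPCs and runs drag-box selection.
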(event Custom|GebäudeBauen
  (params (NameDesGebäudes :type Name))
  (bind _returnvalue (Game|GetPlayerController 0))
  (bind _hitresult (Game|Player|GetHitResultUnderCursorbyChannel _returnvalue "TraceTypeQuery1" true))
  (bind _location (Collision|BreakHitResult _hitresult))
  (bind _returnvalue_2 (Utilities|GetDataTableRow "/Game/RTS/Datenbank/GebäudeDatenbank.GebäudeDatenbank" NameDesGebäudes)
    (:then
      (Variables|Default|SetPlacingBuilding true)
      (Variables|References|SetActualActorMesh (.ActualActor (Utilities|Struct|BreakGebäudeDatenBankStruktur _returnvalue_2)))
      (bind _returnvalue_3 (Game|SpawnActorfromClass "/Game/RTS/Blueprints/BuildingBlueprints/GhostActor.GhostActor_C" (Math|Conversions|ToTransform(Vector) _location) "Undefined" 0 (.GhostActor (Utilities|Struct|BreakGebäudeDatenBankStruktur _returnvalue_2)) (.GeldKosten (Utilities|Struct|BreakGebäudeDatenBankStruktur _returnvalue_2)) (.Holzkosten (Utilities|Struct|BreakGebäudeDatenBankStruktur _returnvalue_2)) (.Steinkosten (Utilities|Struct|BreakGebäudeDatenBankStruktur _returnvalue_2)) (.Metallkosten (Utilities|Struct|BreakGebäudeDatenBankStruktur _returnvalue_2)) (.OverlappingRed (Utilities|Struct|BreakGebäudeDatenBankStruktur _returnvalue_2)) 0))
      (Variables|References|SetGhostBuilding _returnvalue_3)
      (Transformation|SetActorLocation (Variables|References|GetGhostBuilding) _location false false :!label _label)
      (Utilities|FlowControl|Delay 0.01)
      (Utilities|FlowControl|Sequence
        (:then_0
          (Utilities|IsValid (Variables|References|GetGhostBuilding)
            (:Is%20Valid
              (if (Variables|Default|GetPlacingBuilding)
                (goto _label)))
            (:Is%20Not%20Valid
              (Utilities|FlowControl|Gate true) ; enters at Close
            )))
        (:then_1
          (if (Variables|Default|GetPlacingBuilding)
            (Utilities|FlowControl|Gate true) ; enters at Open
            (else
              (Utilities|FlowControl|Gate true) ; enters at Close
            )))))))

(event Custom|PlatziereNutzGebäude)

(event Custom|EntferneAuswahlQuadrat
  (Variables|Default|SetAuswählen? false)
  (Utilities|IsValid (Variables|References|GetAuswahlQuadrat)
    (:Is%20Valid
      (Actor|DestroyActor (Variables|References|GetAuswahlQuadrat)))))

(event Custom|ZieheAuswahlQuadrat
  (Variables|Default|SetAuswählen? true))

(event Custom|ErstelleInfoFenster
  (params (InfoFensterRef :type Informationsfenster%20Object%20Reference) (SpeziNummer :type Integer) (Spezifikation :type String))
  (Variables|Default|SetInfoFensterSpeziNummer SpeziNummer)
  (Default|SetzeInformationen InfoFensterRef Spezifikation)
  (Widget|SetVisibility InfoFensterRef "Visible"))

(event Custom|PlatzierenNichtMöglich?
  (params (GehtEsNicht? :type Boolean))
  (Variables|Default|SetBadTerrain GehtEsNicht?))

(event Custom|PlatziereWohngebäude
  (params (Wohnraum :type Integer) (Kosten :type Integer))
  (bind _mainhudref (Variables|References|GetMainHUDRef))
  (Variables|Daten|SetDukaten (- (Variables|Daten|GetDukaten) Kosten))
  (Variables|Daten|SetVerfügbarerWohnraum Wohnraum)
  (bind (_geld _zufriedenheit _nahrung _verfügbarerwohnraum _benutzterwohnraum) (Default|GetValues _mainhudref))
  (Default|SetValues _mainhudref (Variables|Daten|GetDukaten) _zufriedenheit _nahrung _benutzterwohnraum (+ _verfügbarerwohnraum (Variables|Daten|GetVerfügbarerWohnraum))))

(event Custom|DestroyGhostActor
  (bind _ghostbuilding (Variables|References|GetGhostBuilding))
  (Utilities|IsValid _ghostbuilding
    (:Is%20Valid
      (Actor|DestroyActor _ghostbuilding)
      (Variables|Default|SetPlacingBuilding false))))

(event Custom|FülleInformationsfenster
  (params (InfoWBP :type Vertical%20Box%20Object%20Reference))
  (switch int (Variables|Default|GetInfoFensterSpeziNummer)
    (:0
      (bind _returnvalue (UserInterface|CreateWidget "/Game/RTS/UIS/Regulierung.Regulierung_C" 0 "Steuern"))
      (Widget|Panel|AddChild InfoWBP _returnvalue)
      (bind _returnvalue_2 (UserInterface|CreateWidget "/Game/RTS/UIS/Information.Information_C" 0 "Steuern" "Dukaten" "0"))
      (Widget|Panel|AddChild InfoWBP _returnvalue_2)
      (bind _returnvalue_3 (UserInterface|CreateWidget "/Game/RTS/UIS/Information.Information_C" 0 "Handel" "Dukaten" "0"))
      (Widget|Panel|AddChild InfoWBP _returnvalue_3)
      (bind _returnvalue_4 (UserInterface|CreateWidget "/Game/RTS/UIS/Information.Information_C" 0 "Produktion" "Dukaten" "0"))
      (Widget|Panel|AddChild InfoWBP _returnvalue_4)
      (bind _returnvalue_5 (UserInterface|CreateWidget "/Game/RTS/UIS/Information.Information_C"))
      (Widget|Panel|AddChild InfoWBP _returnvalue_5)
      (bind _returnvalue_6 (UserInterface|CreateWidget "/Game/RTS/UIS/Information.Information_C" 0 "Armee" "Dukaten" "0"))
      (Widget|Panel|AddChild InfoWBP _returnvalue_6)
      (bind _returnvalue_7 (UserInterface|CreateWidget "/Game/RTS/UIS/Information.Information_C" 0 "Gebäude" "Dukaten" "0"))
      (Widget|Panel|AddChild InfoWBP _returnvalue_7))))

(event Custom|SpawnThisNPC
  (params (Type :type NPCType%20Enum :default "NewEnumerator14"))
  (Game|SpawnActorfromClass "/Game/RTS/Blueprints/NPCs/NPC_BP.NPC_BP_C" (Math|Conversions|ToTransform(Vector) (.Location (Collision|BreakHitResult (.HitResult (Game|Player|GetHitResultUnderCursorbyChannel (Game|GetPlayerController 0) "TraceTypeQuery1" true))))) "Undefined" 0 Type 0))

(event Custom|GebäudeAnklicken
  (bind _selectableobjectsenum (Variables|Default|GetSelectableObjectsEnum))
  (bind _hitresult (Class|PlayerController|GetHitResultUnderCursorforObjects _selectableobjectsenum true))
  (bind _hitactor (Collision|BreakHitResult _hitresult))
  (if (!= _hitactor 0)
    (Default|CallHUDRequest _hitactor)))

(event EventBeginPlay
  ;[1 1 1] BeginPlay
  (Utilities|FlowControl|Sequence
    (:then_0
      (Utilities|ReferenceCasts))
    (:then_1
      (bind _asrtsgame_state (Utilities|Casting|CastToRTSGameState (Game|GetGameState)))
      (Variables|References|SetRTSGameState _asrtsgame_state))
    (:then_2
      (Input|SetInputModeGameandUI self 0 "LockOnCapture" false)
      (Utilities|CreateHUDS)
      (UserInterface|Viewport|AddtoViewport (Variables|References|GetMainHUDRef) 0))))

(event EventTick
  (params (DeltaSeconds :type Float%20%28single-precision%29))
  (CallFunction|DragSelect))

(event Input|ActionEvents|InputActionPan
  (params (Key :type Key%20Structure))
  (bind _camerapawnref (Variables|References|GetCameraPawnRef))
  (bind _returnvalue (Transformation|GetActorRotation _camerapawnref))
  (bind (_roll _pitch _yaw) (Math|Rotator|BreakRotator _returnvalue))
  ;[1 1 1] CameraMovement
  ;;[1 1 1] PanY
  (:Pressed
    (Variables|Camera|SetDisableCamNav true)
    (Utilities|FlowControl|Gate true) ; enters at Open
  )
  (:Released
    (Variables|Camera|SetDisableCamNav false)
    (Utilities|FlowControl|Gate true) ; enters at Close
  ))

(event Input|ActionEvents|InputActionZoomReset
  (params (Key :type Key%20Structure))
  ;[1 1 1] CameraMovement
  ;;[1 1 1] Reset Zoom
  (:Pressed
    (Variables|/Script/Engine.SpringArmComponent|SetTargetArmLength (Variables|/Game/RTS/Blueprints/CameraPawn.CameraPawn_C|GetSpringArm (Variables|References|GetCameraPawnRef)) 1.5e+03)))

(event Input|ActionEvents|InputActionPanReset
  (params (Key :type Key%20Structure))
  (bind _camerapawnref (Variables|References|GetCameraPawnRef))
  (bind _returnvalue (Transformation|GetActorRotation _camerapawnref))
  (bind (_roll _pitch _yaw) (Math|Rotator|BreakRotator _returnvalue))
  ;[1 1 1] CameraMovement
  ;;[1 1 1] PanReset
  (:Pressed
    (Transformation|SetActorRotation _camerapawnref (Math|Rotator|MakeRotator _roll 0.0 _yaw))))

(event Input|ActionEvents|InputActionZoomIn
  (params (Key :type Key%20Structure))
  (bind _camerapawnref (Variables|References|GetCameraPawnRef))
  (bind _springarm (Variables|/Game/RTS/Blueprints/CameraPawn.CameraPawn_C|GetSpringArm _camerapawnref))
  ;[1 1 1] CameraMovement
  ;;[1 1 1] Zoom In/Out
  (:Pressed
    (if (not (Variables|Default|GetPlacingBuilding))
      (Variables|/Script/Engine.SpringArmComponent|SetTargetArmLength _springarm (Math|Float|Clamp(Float) (- (Variables|/Script/Engine.SpringArmComponent|GetTargetArmLength _springarm) (Variables|Camera|GetZoomSensitivity)) 5e+02 (Variables|Camera|GetMaxArmDistance))))))

(event Input|ActionEvents|InputActionZoomOut
  (params (Key :type Key%20Structure))
  (bind _camerapawnref (Variables|References|GetCameraPawnRef))
  (bind _springarm (Variables|/Game/RTS/Blueprints/CameraPawn.CameraPawn_C|GetSpringArm _camerapawnref))
  ;[1 1 1] CameraMovement
  ;;[1 1 1] Zoom In/Out
  (:Pressed
    (if (not (Variables|Default|GetPlacingBuilding))
      (Variables|/Script/Engine.SpringArmComponent|SetTargetArmLength _springarm (Math|Float|Clamp(Float) (+ (Variables|Camera|GetZoomSensitivity) (Variables|/Script/Engine.SpringArmComponent|GetTargetArmLength _springarm)) 5e+02 (Variables|Camera|GetMaxArmDistance))))))

(event Input|ActionEvents|InputActionPan
  (params (Key :type Key%20Structure))
  (bind _camerapawnref (Variables|References|GetCameraPawnRef))
  (bind _returnvalue (Transformation|GetActorRotation _camerapawnref))
  (bind (_roll _pitch _yaw) (Math|Rotator|BreakRotator _returnvalue))
  ;[1 1 1] CameraMovement
  ;;[1 1 1] PawnX
  (:Pressed
    (Variables|Camera|SetDisableCamNav true)
    (Utilities|FlowControl|Gate true) ; enters at Open
  )
  (:Released
    (Variables|Camera|SetDisableCamNav false)
    (Utilities|FlowControl|Gate true) ; enters at Close
  ))

(event Input|AxisEvents|InputAxisMoveForward
  (params (AxisValue :type Float%20%28single-precision%29))
  (bind _camerapawnref (Variables|References|GetCameraPawnRef))
  ;[1 1 1] CameraMovement
  ;;[1 1 1] MovementX
  (if (not (Variables|Camera|GetDisableCamNav))
    (Transformation|SetActorTransform _camerapawnref (Utilities|MovementX (CallFunction|MovementSpeedCalculation) (Variables|Camera|GetFastMoveMultiplier) AxisValue _camerapawnref))))

(event Input|AxisEvents|InputAxisMoveRight
  (params (AxisValue :type Float%20%28single-precision%29))
  (bind _movesensitivity (CallFunction|MovementSpeedCalculation))
  (bind _camerapawnref (Variables|References|GetCameraPawnRef))
  (bind _fastmovemultiplier (Variables|Camera|GetFastMoveMultiplier))
  (bind _transform (Utilities|MovementY AxisValue _movesensitivity _fastmovemultiplier _camerapawnref))
  (bind (_location _rotation _scale) (Math|Transform|BreakTransform _transform))
  (bind (_x _y) (Math|Vector|BreakVector _location))
  ;[1 1 1] CameraMovement
  ;;[1 1 1] MovementY
  (if (not (Variables|Camera|GetDisableCamNav))
    (Transformation|SetActorTransform _camerapawnref (Math|Transform|MakeTransform (Math|Vector|MakeVector _x _y (.Z (Math|Vector|BreakVector (Transformation|GetActorLocation _camerapawnref)))) _rotation _scale))))

(event Input|MouseEvents|MouseX
  (params (AxisValue :type Float%20%28single-precision%29))
  (bind _camerapawnref (Variables|References|GetCameraPawnRef))
  (bind _returnvalue (Transformation|GetActorRotation _camerapawnref))
  (bind (_roll _pitch _yaw) (Math|Rotator|BreakRotator _returnvalue))
  ;[1 1 1] CameraMovement
  ;;[1 1 1] PawnX
  (Utilities|FlowControl|Gate true
    (:Exit
      (Transformation|SetActorRotation (Variables|References|GetCameraPawnRef) (Math|Rotator|MakeRotator _roll _pitch (+ _yaw (* (Variables|Camera|GetPanSensitivity) AxisValue)))))))

(event Input|MouseEvents|MouseWheelAxis
  (params (AxisValue :type Float%20%28single-precision%29))
  (bind _ghostbuilding (Variables|References|GetGhostBuilding))
  (if (Variables|Default|GetPlacingBuilding)
    (Utilities|IsValid _ghostbuilding
      (:Is%20Valid
        (bind _output_get (Variables|Default|SetMouseWheelValue (+ (Variables|Default|GetMouseWheelValue) AxisValue)))
        (Transformation|SetActorRotation _ghostbuilding (Math|Rotator|MakeRotator 0.0 0.0 (* _output_get 9e+01)))))
    (else
      (Variables|Default|SetMouseWheelValue 0.0))))

(event Input|MouseEvents|MouseX
  (params (AxisValue :type Float%20%28single-precision%29))
  ;[1 1 1] CameraMovement
  ;;[1 1 1] Movement from Mouse
  (if (not (Variables|Camera|GetDisableCamNav))
    (bind (_deltaxspeed _deltayspeed) (Utilities|ScreenEdgeMovement))
    (Transformation|AddActorLocalOffset (Variables|References|GetCameraPawnRef) (Math|Vector|MakeVector _deltaxspeed _deltayspeed 0.0) true false)))

(event Input|MouseEvents|MouseY
  (params (AxisValue :type Float%20%28single-precision%29))
  ;[1 1 1] CameraMovement
  ;;[1 1 1] Movement from Mouse
  (if (not (Variables|Camera|GetDisableCamNav))
    (Utilities|ScreenEdgeMovement) ; enters at MouseY
  ))

(event Input|MouseEvents|MouseY
  (params (AxisValue :type Float%20%28single-precision%29))
  (bind _camerapawnref (Variables|References|GetCameraPawnRef))
  (bind _returnvalue (Transformation|GetActorRotation _camerapawnref))
  (bind (_roll _pitch _yaw) (Math|Rotator|BreakRotator _returnvalue))
  ;[1 1 1] CameraMovement
  ;;[1 1 1] PanY
  (Utilities|FlowControl|Gate true
    (:Exit
      (Transformation|SetActorRotation (Variables|References|GetCameraPawnRef) (Math|Rotator|MakeRotator _roll (Math|Float|Clamp(Float) (+ _pitch (* (Variables|Camera|GetPanSensitivity) AxisValue)) -15.0 45.0) _yaw)))))

(event Input|KeyboardEvents|LeftShift
  (params (Key :type Key%20Structure))
  ;[1 1 1] CameraMovement
  ;;[1 1 1] Move Multiplier
  (:Pressed
    (Variables|Camera|SetFastMoveMultiplier 2.0))
  (:Released
    (Variables|Camera|SetFastMoveMultiplier 1.0)))

(event Input|KeyboardEvents|P
  (params (Key :type Key%20Structure))
  (:Pressed
    (bind _returnvalue (UserInterface|CreateWidget "/Game/RTS/Blueprints/NPCs/NPCWahl.NPCWahl_C"))
    (Widget|Panel|AddChild (Variables|/Game/RTS/UIS/MainUI_HUD.MainUI_HUD_C|GetInformationen (Variables|References|GetMainHUDRef)) _returnvalue)))

(event Input|KeyboardEvents|Q
  (params (Key :type Key%20Structure))
  (:Pressed
    (Default|ZeitLangsamer (Variables|References|GetMainHUDRef))))

(event Input|MouseEvents|LeftMouseButton
  (params (Key :type Key%20Structure))
  (:Pressed
    (if (Variables|Default|GetPlacingBuilding)
      (Utilities|FlowControl|Gate true
        (:Exit
          (if (not (Variables|Default|GetBadTerrain))
            (Variables|Default|SetPlacingBuilding false)
            (Game|SpawnActorfromClass "/Game/RTS/Blueprints/BuildingBlueprints/GebäudeActor.GebäudeActor_C" (Transformation|GetActorTransform (Variables|References|GetGhostBuilding)) "Undefined" 0 (Variables|References|GetActualActorMesh) (.GeldKosten (Utilities|Struct|BreakGebäudeDatenBankStruktur (stale Custom|GebäudeBauen _returnvalue_2))) (.Holzkosten (Utilities|Struct|BreakGebäudeDatenBankStruktur (stale Custom|GebäudeBauen _returnvalue_2))) (.Steinkosten (Utilities|Struct|BreakGebäudeDatenBankStruktur (stale Custom|GebäudeBauen _returnvalue_2))) (.Metallkosten (Utilities|Struct|BreakGebäudeDatenBankStruktur (stale Custom|GebäudeBauen _returnvalue_2))) (.Wohnraum (Utilities|Struct|BreakGebäudeDatenBankStruktur (stale Custom|GebäudeBauen _returnvalue_2))) (.GebäudeTyp (Utilities|Struct|BreakGebäudeDatenBankStruktur (stale Custom|GebäudeBauen _returnvalue_2))) 0)
            (Actor|DestroyActor (Variables|References|GetGhostBuilding)))))
      (else
        (CallFunction|GebäudeAnklicken)
        (CallFunction|ZieheAuswahlQuadrat))))
  (:Released
    (CallFunction|EntferneAuswahlQuadrat)))

(event Input|KeyboardEvents|SpaceBar
  (params (Key :type Key%20Structure))
  (bind _rtsgamestate (Variables|References|GetRTSGameState))
  (bind _mainhudref (Variables|References|GetMainHUDRef))
  (bind _textblock_14 (Variables|/Game/RTS/UIS/MainUI_HUD.MainUI_HUD_C|GetTextBlock_14 _mainhudref))
  (:Pressed
    (if (Variables|/Game/RTS/GameBPs/RTSGameState.RTSGameState_C|GetStop? _rtsgamestate)
      (Default|TimeGoingon _rtsgamestate)
      (Rendering|Components|TextRender|SetText _textblock_14 "■")
      (else
        (Default|StoppingTime _rtsgamestate)
        (Rendering|Components|TextRender|SetText _textblock_14 "►")))))

(event Input|MouseEvents|RightMouseButton
  (params (Key :type Key%20Structure))
  (:Pressed
    (if (Variables|Default|GetPlacingBuilding)
      (Actor|DestroyActor (Variables|References|GetGhostBuilding))
      (Variables|Default|SetPlacingBuilding false))))

(event Input|KeyboardEvents|E
  (params (Key :type Key%20Structure))
  (:Pressed
    (Default|ZeitSchneller (Variables|References|GetMainHUDRef))))

(fn ConstructionScript)

(fn MovementSpeedCalculation
  (return (Math|Float|Clamp(Float) (/ (Variables|/Script/Engine.SpringArmComponent|GetTargetArmLength (Variables|/Game/RTS/Blueprints/CameraPawn.CameraPawn_C|GetSpringArm (Variables|References|GetCameraPawnRef))) 1e+02) 5.0 2e+01)))

(fn SetSightDistance
  (return (+ (Variables|Camera|GetSightDistance) (Variables|/Script/Engine.SpringArmComponent|GetTargetArmLength (Variables|/Game/RTS/Blueprints/CameraPawn.CameraPawn_C|GetSpringArm (Variables|References|GetCameraPawnRef))))))

(fn ÜberprüfeGeld
  (params (Kosten :type Integer))
  (if (<= Kosten (Variables|Daten|GetDukaten))
    (Variables|Default|SetGenugGeld? true)
    (else
      (Variables|Default|SetGenugGeld? false)))
  (return (Variables|Default|GetGenugGeld?)))

(fn AlleAusgewähltenActors
  (CallFunction|EmptyMinionList)
  (if (>= (Utilities|Array|Length (Collision|GetOverlappingActors (Variables|/Game/RTS/Blueprints/AuswahlFläche/AuswahlQuadrat.AuswahlQuadrat_C|GetCube (Variables|References|GetAuswahlQuadrat)) "/Game/RTS/Blueprints/NPCs/NPC_BP.NPC_BP_C" :!class /Script/Engine.PrimitiveComponent)) 0)
    (for _array_element (Collision|GetOverlappingActors (Variables|/Game/RTS/Blueprints/AuswahlFläche/AuswahlQuadrat.AuswahlQuadrat_C|GetCube (Variables|References|GetAuswahlQuadrat)) "/Game/RTS/Blueprints/NPCs/NPC_BP.NPC_BP_C" :!class /Script/Engine.PrimitiveComponent)
      (bind _ascharacter (Utilities|Casting|CastToCharacter _array_element))
      (CallFunction|AddMiniontoList _ascharacter)))
  (Actor|DestroyActor (Variables|References|GetAuswahlQuadrat))
  (Variables|References|SetAuswahlQuadrat 0))

(fn EmptyMinionList
  (for _array_element (Variables|References|GetCurrentMinion)
    (bind _returnvalue (Rendering|Material|CreateDynamicMaterialInstance (Variables|/Script/Engine.Character|GetMesh _array_element) 0 (Rendering|Material|GetMaterial (Variables|/Script/Engine.Character|GetMesh _array_element) 0) :!class /Script/Engine.PrimitiveComponent))
    (Rendering|Material|SetVectorParameterValue _returnvalue "None" "(R=1.000000,G=1.000000,B=1.000000,A=1.000000)" :!class /Script/Engine.MaterialInstanceDynamic))
  (Utilities|Array|Clear (Variables|References|GetCurrentMinion)))

(fn AddMiniontoList
  (params (NewMinion :type Character%20Object%20Reference))
  (bind _mesh (Variables|/Script/Engine.Character|GetMesh NewMinion))
  (bind _returnvalue (Rendering|Material|CreateDynamicMaterialInstance _mesh 0 (Rendering|Material|GetMaterial _mesh 0) :!class /Script/Engine.PrimitiveComponent))
  (Rendering|Material|SetVectorParameterValue _returnvalue "None" "(R=0.096768,G=0.682292,B=0.093422,A=1.000000)" :!class /Script/Engine.MaterialInstanceDynamic)
  (Utilities|Array|Add (Variables|References|GetCurrentMinion) NewMinion))

(fn DragSelect
  (bind (_position _actor _hashit) (Utilities|MouseHitWorld))
  (if (and (or (!= (Class|Actor|GetInputAxisKeyValue) 0.0) (!= (Class|Actor|GetInputAxisKeyValue) 0.0)) (Variables|Default|GetAuswählen?))
    (Utilities|IsValid (Variables|References|GetAuswahlQuadrat)
      (:Is%20Valid
        (if _hashit
          (Default|ReDrawArea (Variables|References|GetAuswahlQuadrat) _position)))
      (:Is%20Not%20Valid
        (bind _returnvalue (Game|SpawnActorfromClass "/Game/RTS/Blueprints/AuswahlFläche/AuswahlQuadrat.AuswahlQuadrat_C" (Math|Conversions|ToTransform(Vector) _position) "Undefined" 0 0))
        (Variables|References|SetAuswahlQuadrat _returnvalue)
        (Default|ReDrawArea (Variables|References|GetAuswahlQuadrat) _position)))))

(fn SetCalendar
  (params (Date :type Array%20of%20Integers))
  (return false))

(fn SetClock
  (params (Time :type Array%20of%20Integers))
  (return false))