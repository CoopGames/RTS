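; Placement ghost for RTS buildings that previews a building's mesh and tracks its class and construction proxy.
; OnSpawn activates the ghost only when inactive, and KillGhost clears the stored state.
; ConstructBuilding spawns the given class at world origin, then resets the ghost and reloads it from that actor's mesh and proxy.
; SetCalendar and SetClock are stubs returning false.
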(event Custom|OnSpawn
  (params (DisplayMesh :type Static%20Mesh%20Object%20Reference) (BuildingClass :type Building%20Master%20BP%20Class%20Reference) (ConstrucitonProxy :type Construction%20Proxy%20BP%20Class%20Reference))
  (if (not (Variables|Default|GetIsActive?))
    (Variables|Default|SetBuidlingClass BuildingClass)
    (Variables|Default|SetConstructionProxy ConstrucitonProxy)
    (Variables|Default|SetIsActive? true)
    (Variables|Default|SetDisplayMesh DisplayMesh)
    (Components|StaticMesh|SetStaticMesh (Variables|Default|GetGhostBuilding_Mesh) (Variables|Default|GetDisplayMesh))))

(event Custom|KillGhost
  (Variables|Default|SetBuidlingClass 0)
  (Variables|Default|SetConstructionProxy 0)
  (Variables|Default|SetIsActive? false)
  (Variables|Default|SetDisplayMesh 0))

(event EventConstructBuilding
  (params (MainBuilding :type Building%20Master%20BP%20Class%20Reference))
  (bind _returnvalue (Game|SpawnActorfromClass MainBuilding (Math|Transform|MakeTransform "0, 0, 0") "Undefined" 0 (Variables|Default|GetControllerRef) 0))
  (bind _asbuilding_master_bp (Utilities|Casting|CastToBuildingMaster_BPClass MainBuilding))
  (CallFunction|KillGhost)
  (CallFunction|OnSpawn (Variables|/Game/RTS/Blueprints/Buildings/BuildingMaster_BP.BuildingMaster_BP_C|GetDisplayMesh _returnvalue) _asbuilding_master_bp (Variables|/Game/RTS/Blueprints/Buildings/BuildingMaster_BP.BuildingMaster_BP_C|GetConstructionProxy _returnvalue)))

(fn ConstructionScript)

(fn SetCalendar
  (params (Date :type Array%20of%20Integers))
  (return false))

(fn SetClock
  (params (Time :type Array%20of%20Integers))
  (return false))