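; NPC Blueprint for an RTS villager whose profession sets its body color and profile.
; On BeginPlay it creates a dynamic material, tints it by type, builds a profile with a random male name and binds to the RTS camera controller's HUD request.
; ErstelleInfoFenster replaces the HUD info window with this NPC's details when it is the requested actor.
; The selection-square and female-name logic is unconnected.
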(event Custom|ErstelleInfoFenster
  (params (Actor :type Actor%20Object%20Reference))
  (bind _commander (Variables|Default|GetCommander))
  (bind _mainhudref (Variables|/Game/RTS/Blueprints/RTSCameraController.RTSCameraController_C|GetMainHUDRef _commander))
  (if (== Actor self)
    (bind _returnvalue (UserInterface|CreateWidget "/Game/RTS/UIS/NPCInfo.NPCInfo_C" 0 (Variables|Default|GetType) (Variables|Default|GetMyProfile)))
    (Default|LöscheInfoFenster _mainhudref)
    (Widget|Panel|AddChild (Variables|/Game/RTS/UIS/MainUI_HUD.MainUI_HUD_C|GetInformationen _mainhudref) _returnvalue)))

(event EventBeginPlay
  (bind _returnvalue (Rendering|Material|CreateDynamicMaterialInstance (Variables|Character|GetMesh) 0 "/Game/RTS/Character/Materials/M_UE4Man_Body_Inst.M_UE4Man_Body_Inst" :!class /Script/Engine.PrimitiveComponent))
  (Variables|Default|SetMaterialInstance _returnvalue)
  (CallFunction|RandomNPCFeatures (Variables|Default|GetType))
  (bind _asrtscamera_controller (Utilities|Casting|CastToRTSCameraController (Game|GetPlayerController 0)))
  (Variables|Default|SetCommander _asrtscamera_controller)
  (EventDispatchers|BindEventtoHUDRequest (Variables|Default|GetCommander) (EventDispatchers|CreateEvent :!event Custom|ErstelleInfoFenster)))

(event Collision|EventActorBeginOverlap
  (params (OtherActor :type Actor%20Object%20Reference)))

(event EventTick
  (params (DeltaSeconds :type Float%20%28single-precision%29)))

(fn ConstructionScript)

(fn RandomNPCFeatures
  (params (Type :type NPCType%20Enum :default "NewEnumerator14"))
  (bind _materialinstance (Variables|Default|GetMaterialInstance))
  (Variables|Default|SetNPCType Type)
  (switch Utilities|FlowControl|Switch|SwitchonNPCType (Variables|Default|GetNPCType)
    (:NewEnumerator14
      (Rendering|Material|SetVectorParameterValue _materialinstance "BodyColor" "(R=1.000000,G=0.000000,B=0.490836,A=1.000000)" :!class /Script/Engine.MaterialInstanceDynamic))
    (:NewEnumerator0
      (Rendering|Material|SetVectorParameterValue _materialinstance "BodyColor" "(R=1.000000,G=0.902706,B=0.000000,A=1.000000)" :!class /Script/Engine.MaterialInstanceDynamic))
    (:NewEnumerator2
      (Rendering|Material|SetVectorParameterValue _materialinstance "BodyColor" "(R=1.000000,G=0.142180,B=0.000000,A=1.000000)" :!class /Script/Engine.MaterialInstanceDynamic))
    (:NewEnumerator9
      (Rendering|Material|SetVectorParameterValue _materialinstance "BodyColor" "(R=0.006859,G=0.600335,B=1.000000,A=1.000000)" :!class /Script/Engine.MaterialInstanceDynamic))
    (:NewEnumerator3
      (Rendering|Material|SetVectorParameterValue _materialinstance "BodyColor" "(R=0.166667,G=0.166667,B=0.166667,A=1.000000)" :!class /Script/Engine.MaterialInstanceDynamic))
    (:NewEnumerator10
      (Rendering|Material|SetVectorParameterValue _materialinstance "BodyColor" "(R=0.879066,G=1.000000,B=0.354167,A=1.000000)" :!class /Script/Engine.MaterialInstanceDynamic))
    (:NewEnumerator15
      (Rendering|Material|SetVectorParameterValue _materialinstance "BodyColor" "(R=1.000000,G=1.000000,B=1.000000,A=1.000000)" :!class /Script/Engine.MaterialInstanceDynamic))
    (:NewEnumerator11
      (Rendering|Material|SetVectorParameterValue _materialinstance "BodyColor" "(R=1.000000,G=0.016950,B=0.000000,A=1.000000)" :!class /Script/Engine.MaterialInstanceDynamic))
    (:NewEnumerator12
      (Rendering|Material|SetVectorParameterValue _materialinstance "BodyColor" "(R=0.000000,G=1.000000,B=0.056642,A=1.000000)" :!class /Script/Engine.MaterialInstanceDynamic))
    (:NewEnumerator13
      (Rendering|Material|SetVectorParameterValue _materialinstance "BodyColor" "(R=0.005208,G=0.005208,B=0.005208,A=1.000000)" :!class /Script/Engine.MaterialInstanceDynamic))
    (:NewEnumerator16
      (Rendering|Material|SetVectorParameterValue _materialinstance "BodyColor" "(R=0.254050,G=0.255208,B=0.070448,A=1.000000)" :!class /Script/Engine.MaterialInstanceDynamic)))
  (bind _name (CallFunction|GetRandomName "NewEnumerator14"))
  (Variables|Default|SetMyProfile (Utilities|Struct|MakeNPCProfile_struct _name (Variables|Default|GetNPCType)))
  (bind _returnvalue (Rendering|Material|GetVectorParameterValue (Variables|Default|GetMaterialInstance) "BodyColor" :!class /Script/Engine.MaterialInstanceDynamic))
  (Variables|Default|SetBodyColor _returnvalue))

(fn GetRandomName
  (params (Gender :type NPCType%20Enum :default "NewEnumerator14"))
  (return (Utilities|String|EnumtoString (Utilities|Enum|LiteralenumNPCNameMale (Utilities|Enum|ByteToEnumNPCNameMale (Math|Conversions|ToByte(Integer) (Math|Random|RandomIntegerinRange 0 (- (|GetNumEnumEntries) 1))))))))