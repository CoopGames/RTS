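; Game mode for the main menu of an RTS, owning the menu widgets and the screen flow between them.
; On begin play it shows the main menu with UI-only input and a visible cursor; custom events swap in settings or credits, playing camera animations, with settings also handling the return.
; Other events start the game via the game instance's loading screen and map load, or quit behind a confirmation popup.
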(event Custom|Beende%20Spiel
  ;[1 1 1] Beende Spiel
  (Game|QuitGame 0 "Quit"))

(event Custom|Beenden%20Fenster
  ;[1 1 1] Bestätigung zum Beenden des Spiels
  (bind _returnvalue (UserInterface|CreateWidget "/Game/MainMenu/UI/ConfirmClose.ConfirmClose_C"))
  (bind _output_get (Variables|Default|SetConfirmCloseRef _returnvalue))
  (UserInterface|Viewport|AddtoViewport _output_get 0))

(event Custom|StarteSpiel
  ;[1 1 1] Startet Spiel
  (Utilities|IsValid (Variables|Default|GetConfirmCloseRef)
    (:Is%20Valid
      (Widget|RemovefromParent (Variables|Default|GetConfirmCloseRef)))
    (:Is%20Not%20Valid
      _))
  (bind _asrtsgameinstance (Utilities|Casting|CastToRTSGameinstance (Game|GetGameInstance)))
  (Default|ShowLoadingScreen _asrtsgameinstance)
  (Game|OpenLevel(byName) "RTS_Map"))

(event Custom|ErstelleCreditsMenü
  (Utilities|IsValid (Variables|Default|GetConfirmCloseRef)
    (:Is%20Valid
      (Widget|RemovefromParent (Variables|Default|GetConfirmCloseRef)))
    (:Is%20Not%20Valid
      _))
  (Widget|RemovefromParent (Variables|Default|GetHauptmenüRef))
  (bind _returnvalue (UserInterface|CreateWidget "/Game/MainMenu/UI/Credits.Credits_C"))
  (bind _output_get (Variables|Default|SetCreditsmenüRef _returnvalue))
  (UserInterface|Viewport|AddtoViewport _output_get 0)
  (Audio|Components|Audio|Play (Variables|Default|GetCreditsCamera)))

(event Custom|ErstelleHauptmenü
  ;[1 1 1] Hauptmenü erstellen
  (bind _returnvalue (UserInterface|CreateWidget "/Game/MainMenu/UI/MainMenu.MainMenu_C"))
  (bind _output_get (Variables|Default|SetHauptmenüRef _returnvalue))
  (UserInterface|Viewport|AddtoViewport _output_get 0)
  (Input|SetInputModeUIOnly (Game|GetPlayerController 0) (Variables|Default|GetHauptmenüRef) "DoNotLock")
  (Variables|/Script/Engine.PlayerController|SetbShowMouseCursor (Game|GetPlayerController 0) true))

(event Custom|BeendenFensterBeenden
  ;[1 1 1] BeendetDasBeendenFenser
  (Widget|RemovefromParent (Variables|Default|GetConfirmCloseRef)))

(event Custom|VomEinstellungsmenüZurück
  (Widget|RemovefromParent (Variables|Default|GetOptionsmenüRef))
  (Utilities|IsValid (Variables|Default|GetHauptmenüRef)
    (:Is%20Valid
      (UserInterface|Viewport|AddtoViewport (Variables|Default|GetHauptmenüRef) 0))
    (:Is%20Not%20Valid
      (bind _returnvalue (UserInterface|CreateWidget "/Game/MainMenu/UI/MainMenu.MainMenu_C"))
      (bind _output_get (Variables|Default|SetHauptmenüRef _returnvalue))
      (UserInterface|Viewport|AddtoViewport _output_get 0)))
  (Utilities|String|Reverse (Variables|Default|GetSettingsCamera)))

(event Custom|ErstelleOptionsmenü
  ;[1 1 1] Optionsmenü erstellen
  (Utilities|IsValid (Variables|Default|GetConfirmCloseRef)
    (:Is%20Valid
      (Widget|RemovefromParent (Variables|Default|GetConfirmCloseRef)))
    (:Is%20Not%20Valid
      _))
  (Widget|RemovefromParent (Variables|Default|GetHauptmenüRef))
  (bind _returnvalue (UserInterface|CreateWidget "/Game/MainMenu/UI/Settings.Settings_C"))
  (bind _output_get (Variables|Default|SetOptionsmenüRef _returnvalue))
  (UserInterface|Viewport|AddtoViewport _output_get 0)
  (Audio|Components|Audio|Play (Variables|Default|GetSettingsCamera)))

(event EventBeginPlay
  (CallFunction|ErstelleHauptmenü))

(event EventTick
  (params (DeltaSeconds :type Float%20%28single-precision%29)))

(fn ConstructionScript)