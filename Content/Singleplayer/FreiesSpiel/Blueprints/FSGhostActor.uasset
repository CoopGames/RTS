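; Ghost preview actor for a building in the singleplayer free play mode (FreiesSpiel).
; On BeginPlay it sets its static mesh to the GhostActor mesh from GebäudeStruct.
; Tick and overlap events are empty.
; Disconnected leftover logic would set BadTerrain from a money check or swap between the normal and red overlap meshes, but it never runs.
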(event EventBeginPlay
  (Components|StaticMesh|SetStaticMesh (Variables|Debug|GetStaticMeshComponent) (.GhostActor (Utilities|Struct|BreakGebäudeDatenBankStruktur (Variables|Default|GetGebäudeStruct)))))

(event EventTick
  (params (DeltaSeconds :type Float%20%28single-precision%29)))

(event Collision|EventActorBeginOverlap
  (params (OtherActor :type Actor%20Object%20Reference)))

(event Collision|EventActorEndOverlap
  (params (OtherActor :type Actor%20Object%20Reference)))

(fn ConstructionScript)