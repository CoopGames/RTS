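; Building actor for the singleplayer free-play mode (FreiesSpiel), configured through its GebäudeStruct data.
; On BeginPlay it applies the struct's ActualActor as its static mesh, which is its only active logic.
; Disconnected remnants would open a GebäudeInfo widget in the main HUD, bind info-window and HUD-request events, and register residential buildings' housing space and cost with the player controller.
; Overlap, info-window, Tick and construction handlers are empty.
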(event Custom|ErstelleInfofenster
  (params (Actor :type Actor%20Object%20Reference)))

(event EventBeginPlay
  (Components|StaticMesh|SetStaticMesh (Variables|Debug|GetStaticMeshComponent) (.ActualActor (Utilities|Struct|BreakGebäudeDatenBankStruktur (Variables|Default|GetGebäudeStruct)))))

(event Collision|EventActorBeginOverlap
  (params (OtherActor :type Actor%20Object%20Reference)))

(event EventTick
  (params (DeltaSeconds :type Float%20%28single-precision%29)))

(fn ConstructionScript)