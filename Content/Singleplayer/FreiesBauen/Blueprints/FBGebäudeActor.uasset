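; Building actor for the singleplayer free-build mode (FreiesBauen), configured by its GebäudeStruct.
; On BeginPlay it applies the struct's mesh and binds to the Commander's info-window event.
; When that event names this actor, it replaces the main UI's info window with a widget showing the building type.
; InteragiereMitPC switches on building type, but its branches are empty.
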(event Custom|ErstelleInfofenster
  (params (Actor :type Actor%20Object%20Reference))
  (bind _commander (Variables|Default|GetCommander))
  (bind _gamemoderef (Variables|/Game/Singleplayer/FreiesBauen/Blueprints/FreiesBauenPC.FreiesBauenPC_C|GetGamemodeRef _commander))
  (bind _mainuiref (Variables|/Game/Singleplayer/FreiesBauen/Blueprints/FreiesBauenGM.FreiesBauenGM_C|GetMainUIRef _gamemoderef))
  (if (== Actor self)
    (bind _returnvalue (UserInterface|CreateWidget "/Game/Singleplayer/FreiesBauen/UIs/FBInformationsfensterGebäude.FBInformationsfensterGebäude_C" 0 false (Utilities|String|EnumtoString (.GebäudeTyp (Utilities|Struct|BreakGebäudeDatenBankStruktur (Variables|Default|GetGebäudeStruct))))))
    (Default|LöscheInfoFenster _mainuiref)
    (Widget|Panel|AddChild (Variables|/Game/Singleplayer/FreiesBauen/UIs/FBMainUI.FBMainUI_C|GetInfoBox _mainuiref) _returnvalue)))

(event EventBeginPlay
  (Components|StaticMesh|SetStaticMesh (Variables|Debug|GetStaticMeshComponent) (.ActualActor (Utilities|Struct|BreakGebäudeDatenBankStruktur (Variables|Default|GetGebäudeStruct))))
  (EventDispatchers|BindEventtoErstelleInfoFenster (Variables|Default|GetCommander) (EventDispatchers|CreateEvent :!event Custom|ErstelleInfofenster))
  (CallFunction|InteragiereMitPC))

(event Collision|EventActorBeginOverlap
  (params (OtherActor :type Actor%20Object%20Reference)))

(event EventTick
  (params (DeltaSeconds :type Float%20%28single-precision%29)))

(fn ConstructionScript)

(fn InteragiereMitPC
  (switch Utilities|FlowControl|Switch|SwitchonGebäudeTypes (.GebäudeTyp (Utilities|Struct|BreakGebäudeDatenBankStruktur (Variables|Default|GetGebäudeStruct)))))