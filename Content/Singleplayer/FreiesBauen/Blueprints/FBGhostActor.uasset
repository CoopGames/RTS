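; Placement ghost for singleplayer free building, previewing the building from GebäudeStruct.
; BeginPlay applies the ghost mesh; overlaps swap it to the red variant and set the player controller's BadTerrain.
; Two cross-resetting DoOnce nodes alternate the states, restoring mesh and flag on the first end overlap.
; Tick also rewrites BadTerrain every frame from the controller's resource check, overriding the overlap result.
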(event EventBeginPlay
  (Components|StaticMesh|SetStaticMesh (Variables|Debug|GetStaticMeshComponent) (.GhostActor (Utilities|Struct|BreakGebäudeDatenBankStruktur (Variables|Default|GetGebäudeStruct)))))

(event EventTick
  (params (DeltaSeconds :type Float%20%28single-precision%29))
  (bind _freiesbauenpcref (Variables|Default|GetFreiesBauenPCRef))
  (bind _kanngebautwerden_ (Default|ÜberprüfeRohstoffe (Variables|Default|GetFreiesBauenPCRef) (Variables|Default|GetGebäudeStruct)))
  (if _kanngebautwerden_
    (Variables|/Game/Singleplayer/FreiesBauen/Blueprints/FreiesBauenPC.FreiesBauenPC_C|SetBadTerrain _freiesbauenpcref false)
    (else
      (Variables|/Game/Singleplayer/FreiesBauen/Blueprints/FreiesBauenPC.FreiesBauenPC_C|SetBadTerrain _freiesbauenpcref true))))

(event Collision|EventActorBeginOverlap
  (params (OtherActor :type Actor%20Object%20Reference))
  (bind _gebäudestruct (Variables|Default|GetGebäudeStruct))
  (bind (_gebäudetyp _geldkosten _wohnraum _holzkosten _lehmkosten _steinkosten _marmorkosten _eisenkosten _bronzekosten _ghostactor _actualactor _overlappingred) (Utilities|Struct|BreakGebäudeDatenBankStruktur _gebäudestruct))
  (Utilities|FlowControl|DoOnce false
    (:Completed
      (Components|StaticMesh|SetStaticMesh (Variables|Debug|GetStaticMeshComponent) _overlappingred)
      (Variables|/Game/Singleplayer/FreiesBauen/Blueprints/FreiesBauenPC.FreiesBauenPC_C|SetBadTerrain (Variables|Default|GetFreiesBauenPCRef) true)
      (Utilities|FlowControl|DoOnce false) ; enters at Reset
    )))

(event Collision|EventActorEndOverlap
  (params (OtherActor :type Actor%20Object%20Reference))
  (bind _gebäudestruct (Variables|Default|GetGebäudeStruct))
  (bind (_gebäudetyp _geldkosten _wohnraum _holzkosten _lehmkosten _steinkosten _marmorkosten _eisenkosten _bronzekosten _ghostactor _actualactor _overlappingred) (Utilities|Struct|BreakGebäudeDatenBankStruktur _gebäudestruct))
  (Utilities|FlowControl|DoOnce false
    (:Completed
      (Components|StaticMesh|SetStaticMesh (Variables|Debug|GetStaticMeshComponent) _ghostactor)
      (Variables|/Game/Singleplayer/FreiesBauen/Blueprints/FreiesBauenPC.FreiesBauenPC_C|SetBadTerrain (Variables|Default|GetFreiesBauenPCRef) false)
      (Utilities|FlowControl|DoOnce false) ; enters at Reset
    )))

(fn ConstructionScript)