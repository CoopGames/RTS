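; Singleplayer free-build (Freies Bauen) player controller that drives the camera pawn and handles building placement.
; Camera supports axis and screen-edge movement, spring-arm zoom and gated pan rotation, with axis movement speed scaled by zoom.
; BaueGebäude spawns a ghost from a data table row that follows the cursor via a Delay loop, with wheel rotation, click-to-place on valid terrain and right-click cancel.
; GebäudeAnklicken opens info windows for clicked objects.
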(event Custom|BaueGebäude
  (params (NameDesGebäudes :type Name))
  (bind _returnvalue (Game|GetPlayerController 0))
  (bind _hitresult (Game|Player|GetHitResultUnderCursorbyChannel _returnvalue "TraceTypeQuery1" true))
  (bind _location (Collision|BreakHitResult _hitresult))
  (bind _returnvalue_2 (Utilities|GetDataTableRow "/Game/RTS/Datenbank/GebäudeDatenbank.GebäudeDatenbank" NameDesGebäudes)
    (:then
      (Variables|Default|SetPlacingBuilding true)
      (bind _returnvalue_3 (Game|SpawnActorfromClass "/Game/Singleplayer/FreiesBauen/Blueprints/FBGhostActor.FBGhostActor_C" (Math|Conversions|ToTransform(Vector) _location) "Undefined" 0 self _returnvalue_2 true 2 0))
      (Variables|Default|SetGhostActorRef _returnvalue_3)
      (Transformation|SetActorLocation _location false false :!label _label)
      (Utilities|FlowControl|Delay 0.01)
      (Utilities|IsValid (Variables|Default|GetGhostActorRef)
        (:Is%20Valid
          (if (Variables|Default|GetPlacingBuilding)
            (Utilities|FlowControl|Sequence
              (:then_0
                (goto _label))
              (:then_1
                (if (Variables|Default|GetPlacingBuilding)
                  (Utilities|FlowControl|Gate true) ; enters at Open
                  (else
                    (Utilities|FlowControl|Gate true) ; enters at Close
                  ))))))))))

(event Custom|GebäudeAnklicken
  (bind _selectableobjects (Variables|Default|GetSelectableObjects))
  (bind _hitresult (Class|PlayerController|GetHitResultUnderCursorforObjects _selectableobjects true))
  (bind _hitactor (Collision|BreakHitResult _hitresult))
  (if (!= _hitactor 0)
    (Default|CallErstelleInfoFenster _hitactor)))

(event EventBeginPlay
  (Utilities|ReferenceCasts))

(event EventTick
  (params (DeltaSeconds :type Float%20%28single-precision%29)))

(event Input|ActionEvents|InputActionPanReset
  (params (Key :type Key%20Structure))
  (bind _camerapawnref (Variables|Camera|GetCameraPawnRef))
  (bind _returnvalue (Transformation|GetActorRotation _camerapawnref))
  (bind (_roll _pitch _yaw) (Math|Rotator|BreakRotator _returnvalue))
  ;[1 1 1] Camera Movement
  (:Pressed
    (Transformation|SetActorRotation _camerapawnref (Math|Rotator|MakeRotator _roll 0.0 _yaw))))

(event Input|ActionEvents|InputActionZoomIn
  (params (Key :type Key%20Structure))
  (bind _camerapawnref (Variables|Camera|GetCameraPawnRef))
  (bind _springarm (Variables|/Game/RTS/Blueprints/CameraPawn.CameraPawn_C|GetSpringArm _camerapawnref))
  ;[1 1 1] Camera Movement
  ;;[1 1 1] Zooming
  (:Pressed
    (if (not (Variables|Default|GetPlacingBuilding))
      (Variables|/Script/Engine.SpringArmComponent|SetTargetArmLength _springarm (Math|Float|Clamp(Float) (- (Variables|/Script/Engine.SpringArmComponent|GetTargetArmLength _springarm) (Variables|Camera|GetZoomSensitivity)) 5e+02 (Variables|Camera|GetMaxArmDistance))))))

(event Input|ActionEvents|InputActionPan
  (params (Key :type Key%20Structure))
  (bind _camerapawnref (Variables|Camera|GetCameraPawnRef))
  (bind _returnvalue (Transformation|GetActorRotation _camerapawnref))
  (bind (_roll _pitch _yaw) (Math|Rotator|BreakRotator _returnvalue))
  ;[1 1 1] Camera Movement
  (:Pressed
    (Variables|Camera|SetDisableCamNav true)
    (Utilities|FlowControl|Gate true) ; enters at Open
  )
  (:Released
    (Variables|Camera|SetDisableCamNav false)
    (Utilities|FlowControl|Gate true) ; enters at Close
  ))

(event Input|ActionEvents|InputActionZoomOut
  (params (Key :type Key%20Structure))
  (bind _camerapawnref (Variables|Camera|GetCameraPawnRef))
  (bind _springarm (Variables|/Game/RTS/Blueprints/CameraPawn.CameraPawn_C|GetSpringArm _camerapawnref))
  ;[1 1 1] Camera Movement
  ;;[1 1 1] Zooming
  (:Pressed
    (if (not (Variables|Default|GetPlacingBuilding))
      (Variables|/Script/Engine.SpringArmComponent|SetTargetArmLength _springarm (Math|Float|Clamp(Float) (+ (Variables|Camera|GetZoomSensitivity) (Variables|/Script/Engine.SpringArmComponent|GetTargetArmLength _springarm)) 5e+02 (Variables|Camera|GetMaxArmDistance))))))

(event Input|ActionEvents|InputActionZoomReset
  (params (Key :type Key%20Structure))
  ;[1 1 1] Camera Movement
  ;;[1 1 1] Zooming
  (:Pressed
    (Variables|/Script/Engine.SpringArmComponent|SetTargetArmLength (Variables|/Game/RTS/Blueprints/CameraPawn.CameraPawn_C|GetSpringArm (Variables|Camera|GetCameraPawnRef)) 1.5e+03)))

(event Input|ActionEvents|InputActionPan
  (params (Key :type Key%20Structure))
  (bind _camerapawnref (Variables|Camera|GetCameraPawnRef))
  (bind _returnvalue (Transformation|GetActorRotation _camerapawnref))
  (bind (_roll _pitch _yaw) (Math|Rotator|BreakRotator _returnvalue))
  ;[1 1 1] Camera Movement
  (:Pressed
    (Variables|Camera|SetDisableCamNav true)
    (Utilities|FlowControl|Gate true) ; enters at Open
  )
  (:Released
    (Variables|Camera|SetDisableCamNav false)
    (Utilities|FlowControl|Gate true) ; enters at Close
  ))

(event Input|AxisEvents|InputAxisMoveForward
  (params (AxisValue :type Float%20%28single-precision%29))
  (bind _camerapawnref (Variables|Camera|GetCameraPawnRef))
  ;[1 1 1] Camera Movement
  (Utilities|ReferenceCasts)
  (if (not (Variables|Camera|GetDisableCamNav))
    (Transformation|SetActorTransform _camerapawnref (Utilities|MovementX (CallFunction|MovementSpeedCalculation) (Variables|Camera|GetFastMoveMultiplier) AxisValue _camerapawnref))))

(event Input|AxisEvents|InputAxisMoveRight
  (params (AxisValue :type Float%20%28single-precision%29))
  (bind _movesensitivity (CallFunction|MovementSpeedCalculation))
  (bind _camerapawnref (Variables|Camera|GetCameraPawnRef))
  (bind _fastmovemultiplier (Variables|Camera|GetFastMoveMultiplier))
  (bind _transform (Utilities|MovementY AxisValue _movesensitivity _fastmovemultiplier _camerapawnref))
  (bind (_location _rotation _scale) (Math|Transform|BreakTransform _transform))
  (bind (_x _y) (Math|Vector|BreakVector _location))
  ;[1 1 1] Camera Movement
  (Utilities|ReferenceCasts)
  (if (not (Variables|Camera|GetDisableCamNav))
    (Transformation|SetActorTransform _camerapawnref (Math|Transform|MakeTransform (Math|Vector|MakeVector _x _y 0.0) _rotation _scale))))

(event Input|MouseEvents|MouseX
  (params (AxisValue :type Float%20%28single-precision%29))
  ;[1 1 1] Camera Movement
  ;;[1 1 1] Camera mouse edge movement
  (Utilities|ReferenceCasts)
  (if (not (Variables|Camera|GetDisableCamNav))
    (bind (_deltaxspeed _deltayspeed) (Utilities|ScreenEdgeMovement))
    (Transformation|AddActorLocalOffset (Variables|Camera|GetCameraPawnRef) (Math|Vector|MakeVector _deltaxspeed _deltayspeed 0.0) false false)))

(event Input|MouseEvents|MouseY
  (params (AxisValue :type Float%20%28single-precision%29))
  ;[1 1 1] Camera Movement
  ;;[1 1 1] Camera mouse edge movement
  (Utilities|ReferenceCasts)
  (if (not (Variables|Camera|GetDisableCamNav))
    (Utilities|ScreenEdgeMovement) ; enters at MouseY
  ))

(event Input|MouseEvents|MouseWheelAxis
  (params (AxisValue :type Float%20%28single-precision%29))
  (if (Variables|Default|GetPlacingBuilding)
    (Utilities|IsValid 0
      (:Is%20Valid
        (bind _output_get (Variables|Default|SetMouseWheelValue (+ (Variables|Default|GetMouseWheelValue) AxisValue)))
        (Transformation|SetActorRotation (Math|Rotator|MakeRotator 0.0 0.0 (* _output_get 9e+01)))))
    (else
      (Variables|Default|SetMouseWheelValue 0.0))))

(event Input|MouseEvents|MouseX
  (params (AxisValue :type Float%20%28single-precision%29))
  (bind _camerapawnref (Variables|Camera|GetCameraPawnRef))
  (bind _returnvalue (Transformation|GetActorRotation _camerapawnref))
  (bind (_roll _pitch _yaw) (Math|Rotator|BreakRotator _returnvalue))
  ;[1 1 1] Camera Movement
  (Utilities|FlowControl|Gate true
    (:Exit
      (Transformation|SetActorRotation (Variables|Camera|GetCameraPawnRef) (Math|Rotator|MakeRotator _roll _pitch (+ _yaw (* (Variables|Camera|GetPanSensitivity) AxisValue)))))))

(event Input|MouseEvents|MouseY
  (params (AxisValue :type Float%20%28single-precision%29))
  (bind _camerapawnref (Variables|Camera|GetCameraPawnRef))
  (bind _returnvalue (Transformation|GetActorRotation _camerapawnref))
  (bind (_roll _pitch _yaw) (Math|Rotator|BreakRotator _returnvalue))
  ;[1 1 1] Camera Movement
  (Utilities|FlowControl|Gate true
    (:Exit
      (Transformation|SetActorRotation (Variables|Camera|GetCameraPawnRef) (Math|Rotator|MakeRotator _roll (Math|Float|Clamp(Float) (+ _pitch (* (Variables|Camera|GetPanSensitivity) AxisValue)) -15.0 45.0) _yaw)))))

(event Input|KeyboardEvents|LeftShift
  (params (Key :type Key%20Structure))
  ;[1 1 1] Camera Movement
  (:Pressed
    (Variables|Camera|SetFastMoveMultiplier 0.0))
  (:Released
    (Variables|Camera|SetFastMoveMultiplier 1.0)))

(event Input|MouseEvents|LeftMouseButton
  (params (Key :type Key%20Structure))
  (:Pressed
    (if (Variables|Default|GetPlacingBuilding)
      (Utilities|FlowControl|Gate true
        (:Exit
          (if (not (Variables|Default|GetBadTerrain))
            (Variables|Default|SetPlacingBuilding false)
            (Game|SpawnActorfromClass "/Game/Singleplayer/FreiesBauen/Blueprints/FBGebäudeActor.FBGebäudeActor_C" (Transformation|GetActorTransform) "Undefined" 0 0 (stale Custom|BaueGebäude _returnvalue_2) 0)
            (Actor|DestroyActor)))))))

(event Input|MouseEvents|RightMouseButton
  (params (Key :type Key%20Structure))
  (:Pressed
    (if (Variables|Default|GetPlacingBuilding)
      (Actor|DestroyActor)
      (Variables|Default|SetPlacingBuilding false))))

(fn ConstructionScript)

(fn MovementSpeedCalculation
  (return (Math|Float|Clamp(Float) (/ (Variables|/Script/Engine.SpringArmComponent|GetTargetArmLength (Variables|/Game/RTS/Blueprints/CameraPawn.CameraPawn_C|GetSpringArm (Variables|Camera|GetCameraPawnRef))) 1e+02) 5.0 2e+01)))