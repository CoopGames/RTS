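; Troop Blueprint for the singleplayer free-build mode that holds a unit's stats and military boosts.
; TruppenSpawnen looks up a named row in the TruppenDatenbank data table and stores each base stat plus its accumulated boost, along with upgrade tier, special and skeletal mesh.
; MilitärBoostsActivated adds a boost to the chosen stat in the MilitärBoosts struct, affecting only later TruppenSpawnen calls.
; Despite its name, TruppenSpawnen only sets variables and spawns nothing.
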(event EventBeginPlay)

(event Collision|EventActorBeginOverlap
  (params (OtherActor :type Actor%20Object%20Reference)))

(event EventTick
  (params (DeltaSeconds :type Float%20%28single-precision%29)))

(fn ConstructionScript)

(fn TruppenSpawnen
  (params (Name :type String))
  (bind _militärboosts (Variables|Default|GetMilitärBoosts))
  (bind (_hpboost _dmgboost _reichweiteboost _angriffsgeschwindigkeitboost _geschwindigkeitboost _unterhaltboost) (Utilities|Struct|BreakTruppenBoosts _militärboosts))
  (bind _returnvalue (Utilities|GetDataTableRow "/Game/RTS/Datenbank/TruppenDatenbank.TruppenDatenbank" (Utilities|String|StringToName Name))
    (:then
      (Variables|Default|SetHP (+ _hpboost (.HP (Utilities|Struct|BreakArmeeProfil _returnvalue))))
      (Variables|Default|SetDmg (+ _dmgboost (.DM (Utilities|Struct|BreakArmeeProfil _returnvalue))))
      (Variables|Default|SetReichweite (+ _reichweiteboost (.Reichweite (Utilities|Struct|BreakArmeeProfil _returnvalue))))
      (Variables|Default|SetAngriffsgeschwindigkeit (+ _angriffsgeschwindigkeitboost (.AngriffsGeschwindigkeit (Utilities|Struct|BreakArmeeProfil _returnvalue))))
      (Variables|Default|SetGeschwindigkeit (+ _geschwindigkeitboost (.Geschwindigkeit (Utilities|Struct|BreakArmeeProfil _returnvalue))))
      (Variables|Default|SetUnterhalt+ (+ _unterhaltboost (.Unterhalt (Utilities|Struct|BreakArmeeProfil _returnvalue))))
      (Variables|Default|SetUpgradeStufe (.UpgradeStufe (Utilities|Struct|BreakArmeeProfil _returnvalue)))
      (Variables|Default|SetSpecial (.Special (Utilities|Struct|BreakArmeeProfil _returnvalue)))
      (Variables|Default|Setskeletalmesh (.SkeletalMesh (Utilities|Struct|BreakArmeeProfil _returnvalue))))))

(fn MilitärBoostsActivated
  (params (Truppenwert :type Truppenwerte%20Enum :default "NewEnumerator7") (Boost :type Integer))
  (bind _militärboosts (Variables|Default|GetMilitärBoosts))
  (bind (_hpboost _dmgboost _reichweiteboost _angriffsgeschwindigkeitboost _geschwindigkeitboost _unterhaltboost) (Utilities|Struct|BreakTruppenBoosts _militärboosts))
  (switch Utilities|FlowControl|Switch|SwitchonTruppenwerte Truppenwert
    (:NewEnumerator0
      (Utilities|Struct|SetmembersinTruppenBoosts _militärboosts (+ _hpboost Boost)))
    (:NewEnumerator1
      (Utilities|Struct|SetmembersinTruppenBoosts _militärboosts 0 (+ _dmgboost Boost)))
    (:NewEnumerator2
      (Utilities|Struct|SetmembersinTruppenBoosts _militärboosts 0 0 (+ _reichweiteboost Boost)))
    (:NewEnumerator3
      (Utilities|Struct|SetmembersinTruppenBoosts _militärboosts 0 0 0 (+ _angriffsgeschwindigkeitboost Boost)))
    (:NewEnumerator4
      (Utilities|Struct|SetmembersinTruppenBoosts _militärboosts 0 0 0 0 (+ _geschwindigkeitboost Boost)))
    (:NewEnumerator5
      (Utilities|Struct|SetmembersinTruppenBoosts _militärboosts 0 0 0 0 0 (+ _unterhaltboost Boost)))))